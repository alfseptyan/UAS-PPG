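; BP_NPC is an AI character that can save and restore its state through checkpoints.
; On BeginPlay it finds the component matching its AIBehaviour class, takes that component's SightRangeClass as its AI controller class and spawns that controller.
; GetCheckpointData packages object name, transform and behaviour; SetCheckpointData restores transform and behaviour when the name matches, without respawning the controller.
; Both checkpoint paths print the transform.
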(event `self.ReceiveBeginPlay`
  (set `self.AIControllerClass` (`/Game/Characters/AI/AIBehaviour.SightRangeClass` (`self.GetComponentByClass` "/Game/Characters/AI/AIBehaviour.AIBehaviour_C")))
  (`self.SpawnDefaultController`))

(event `/Game/Checkpoint/BPI_Checkpointable.SetCheckpointData`
  (params (CheckpointData :type "/Game/Checkpoint/S_CheckpointData Structure"))
  (bind (_checkpointableobjectname _bp_npc _objecttransform _npc_aibehavior) (break `/Game/Checkpoint/S_CheckpointData` CheckpointData))
  (if (`KismetStringLibrary.EqualEqual_StrStr` _checkpointableobjectname (`KismetSystemLibrary.GetObjectName` self))
    (`self.K2_SetActorTransform` self _objecttransform false false)
    (set `self.AIBehaviour` _npc_aibehavior)
    (`KismetSystemLibrary.PrintString` (`KismetStringLibrary.Conv_TransformToString` _objecttransform))))

(fn `GetCheckpointData`
  (returns (CheckpointData :type "/Game/Checkpoint/S_CheckpointData Structure"))
  (locals (NewLocalVar :type "Transform Structure"))
  (bind _output_get (set `local.NewLocalVar` (`self.GetTransform` self)))
  (`KismetSystemLibrary.PrintString` (`KismetStringLibrary.Conv_TransformToString` _output_get))
  (return (make `/Game/Checkpoint/S_CheckpointData` (`KismetSystemLibrary.GetObjectName` self) self _output_get (`self.AIBehaviour`))))

(fn `UserConstructionScript`)