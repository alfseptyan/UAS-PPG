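; BP_Door is an interactable, one-time interior door that requires items from the player's inventory.
; Interact checks RequiredItems against BP_PlayerInventory's CarriedItems through CanPlayerOpen.
; On success, it plays the door animation and fade widget, pauses player input, then teleports the player to an offset along the mesh's right vector.
; Otherwise, it briefly shows a debounced Indonesian warning listing all required items, formatted by RequiredItemsInString.
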(event `/Game/ThirdPerson/Blueprints/BPI_Interactable.Interact`
  (bind _returnvalue (`GameplayStatics.GetPlayerController` 0))
  (bind _returnvalue_2 (`GameplayStatics.GetPlayerCharacter` 0))
  (if (not (`self.AlreadyOpened`))
    (bind _canopen (`self.CanPlayerOpen`))
    (if _canopen
      (`SkeletalMeshComponent.PlayAnimation` (`self.SkeletalMesh`) "/Game/Interior/Door/Door_Anim.Door_Anim" false)
      (`self.DisableInput` _returnvalue_2 _returnvalue)
      (bind _returnvalue_3 (`|CreateWidget` "/Game/UI/WBP_DoorFade.WBP_DoorFade_C"))
      (`UserWidget.AddToViewport` _returnvalue_3 0)
      (`KismetSystemLibrary.Delay` 3.0)
      (`self.EnableInput` _returnvalue_2 _returnvalue)
      (`self.K2_SetActorLocation` (`GameplayStatics.GetPlayerCharacter` 0) (+ (* (`SceneComponent.GetRightVector` (`self.SkeletalMesh`)) (100.0 100.0 0.0)) (`self.K2_GetActorLocation`)) false false)
      (set `self.AlreadyOpened` true)
      (elif (not (`self.WarningShown`))
        (bind _returnvalue_4 (`|CreateWidget` "/Game/UI/WBP_InteractWarning.WBP_InteractWarning_C"))
        (bind _widget (`/Game/UI/WBP_InteractWarning.SetWarningText` _returnvalue_4 (`KismetStringLibrary.Concat_StrStr` "Membutuhkan Item: " (`self.RequiredItemsInString`))))
        (bind _output_get (set `self.WarningWidget` _widget))
        (`UserWidget.AddToViewport` _widget 0)
        (set `self.WarningShown` true)
        (`KismetSystemLibrary.Delay` 2.0)
        (`Widget.RemoveFromParent` _output_get)
        (`KismetSystemLibrary.Delay` 0.2)
        (set `self.WarningShown` false)))))

(fn `CanPlayerOpen`
  (returns (CanOpen :type Boolean))
  (locals (CarriedByPlayer :type Boolean :default true))
  (for _array_element (`self.RequiredItems`)
    (if (not (`KismetArrayLibrary.Array_Contains` (`/Game/ThirdPerson/Blueprints/BP_PlayerInventory.CarriedItems` (`self.GetComponentByClass` (`GameplayStatics.GetPlayerPawn` 0) "/Game/ThirdPerson/Blueprints/BP_PlayerInventory.BP_PlayerInventory_C")) _array_element))
      (set `local.CarriedByPlayer` false)
      (break)))
  (return (`local.CarriedByPlayer`)))

(fn `RequiredItemsInString`
  (returns (ResultString :type String))
  (locals (Result :type String) (ArrLength :type Integer))
  (bind _requireditems (`self.RequiredItems`))
  (set `local.ArrLength` (`KismetArrayLibrary.Array_Length` (`self.RequiredItems`)))
  (if (== (`local.ArrLength`) 0)
    (bind _output_get (set `local.Result` ""))
    (return _output_get)
    (elif (== (`local.ArrLength`) 1)
      (bind _output_get_2 (set `local.Result` (`/Game/ThirdPerson/Blueprints/BP_CollectibleItem.Name` (`|GetArrayItem` (`self.RequiredItems`)))))
      (return _output_get_2)
      (elif (== (`local.ArrLength`) 2)
        (bind _output_get_3 (set `local.Result` (`KismetStringLibrary.Concat_StrStr` (`/Game/ThirdPerson/Blueprints/BP_CollectibleItem.Name` (`|GetArrayItem` (`self.RequiredItems`))) " dan " (`/Game/ThirdPerson/Blueprints/BP_CollectibleItem.Name` (`|GetArrayItem` (`self.RequiredItems`) 1)))))
        (return _output_get_3)
        (else
          (for _index (range (+ (- (`local.ArrLength`) 3) 1))
            (set `local.Result` (`KismetStringLibrary.Concat_StrStr` (`local.Result`) (`/Game/ThirdPerson/Blueprints/BP_CollectibleItem.Name` (`|GetArrayItem` (`self.RequiredItems`) _index)) ", ")))
          (bind _output_get_4 (set `local.Result` (`KismetStringLibrary.Concat_StrStr` (`local.Result`) " " (`/Game/ThirdPerson/Blueprints/BP_CollectibleItem.Name` (`|GetArrayItem` (`self.RequiredItems`) (- (`local.ArrLength`) 2))) " dan " (`/Game/ThirdPerson/Blueprints/BP_CollectibleItem.Name` (`|GetArrayItem` _requireditems (`KismetArrayLibrary.Array_LastIndex` _requireditems))))))
          (return _output_get_4))))))

(fn `UserConstructionScript`)